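; Procedural terrain builder, parented to BP_GameBoard, that scatters random BP_Terrain pieces across the board.
; BeginPlay only caches board bounds; ResetTerrain clears terrain and pieces, then runs setup and cleanup.
; Random, Mirror and Double Mirror modes spawn pieces, with temporary BP_Blocker walls through the center for mirrored layouts, duplicated using negated scale.
; Cleanup deletes actors outside hard-coded limits, independent of the cached bounds; ApplyClearance is an unwired stub.
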(event Custom|SetNumberOfSpawnedTerrain
  (params (NumOfTerrain :type Integer))
  (Variables|Default|SetNumberOfTerrain NumOfTerrain))

(event EventBeginPlay
  (CallFunction|SetBounds))

(fn ConstructionScript)

(fn SetupTerrain
  (Utilities|Casting|CastToBP_GameBoard (Actor|GetParentActor)
    (:then
      (Utilities|FlowControl|Sequence
        (:then_0
          (switch Utilities|FlowControl|Switch|SwitchonE_BuilderSetupMode (Variables|Default|GetSetupMode)
            (:NewEnumerator0
              (CallFunction|RandomTerrainPlacement))
            (:NewEnumerator1
              (CallFunction|MirrorTerrainPlacement))
            (:NewEnumerator3
              (CallFunction|DoubleMirrorTerrainPlacement)))
          (CallFunction|RemoveBlockers))
        (:then_1
          (bind _outactors (Actor|GetAllActorsOfClass "/Game/SceneBuilder/BP_Terrain.BP_Terrain_C"))
          (for _array_element _outactors
            (Default|DestroyCollisionBox _array_element)))))
    (:CastFailed
      (Development|PrintString "ERROR<BP_TerrainBuilder>: Parent object type of BP_TerrainBuilder invalid"))))

(fn PlaceSingleTerrain
  (Game|SpawnActorfromClass "/Game/SceneBuilder/BP_Terrain.BP_Terrain_C" (Utilities|GetRandomPointonTopOfTransform) "Undefined" 0 (Utilities|GetRandomTerrainPiece) 0))

(fn ResetTerrain
  (bind _outactors (Actor|GetAllActorsOfClass "/Game/SceneBuilder/BP_Terrain.BP_Terrain_C"))
  (for _array_element _outactors
    (Actor|DestroyActor _array_element))
  (bind _outactors_2 (Actor|GetAllActorsOfClass "/Game/SceneBuilder/Piece/BP_Piece.BP_Piece_C"))
  (for _array_element_2 _outactors_2
    (Actor|DestroyActor _array_element_2))
  (CallFunction|SetBounds)
  (CallFunction|SetupTerrain)
  (CallFunction|CleanupTerrain))

(fn ApplyClearance)

(fn SetBounds
  (bind _returnvalue (Actor|GetParentActor))
  (bind _returnvalue_2 (Transformation|GetActorTransform _returnvalue))
  (bind _asbp_game_board (Utilities|Casting|CastToBP_GameBoard _returnvalue)
    (:then
      (Variables|Default|SetBoundOrigin (.location _returnvalue_2))
      (Variables|Default|SetBoundX (* (Variables|/Game/SceneBuilder/BP_GameBoard.BP_GameBoard_C|GetBOARD_SIZE_X _asbp_game_board) (.x (.scale _returnvalue_2))))
      (Variables|Default|SetBoundY (* (Variables|/Game/SceneBuilder/BP_GameBoard.BP_GameBoard_C|GetBOARD_SIZE_Y _asbp_game_board) (.y (.scale _returnvalue_2)))))
    (:CastFailed
      (Development|PrintString "ERROR<BP_TerrainBuilder>: Parent object type of BP_TerrainBuilder invalid"))))

(fn DEBUGSetOriginArrow
  (Transformation|SetWorldLocation (Variables|Default|GetArrow) (- (Variables|Default|GetBoundOrigin) (Math|Vector|MakeVector (/ (Variables|Default|GetBoundX) 2.0) 0.0 0.0)) false false))

(fn RandomTerrainPlacement
  (for _index (range 0 (Variables|Default|GetNumberOfTerrain))
    (CallFunction|PlaceSingleTerrain)))

(fn MirrorTerrainPlacement
  (Utilities|FlowControl|Sequence
    (:then_0
      (Game|SpawnActorfromClass "/Game/SceneBuilder/BP_Blocker.BP_Blocker_C" (Math|Transform|MakeTransform (Variables|Default|GetBoundOrigin) "0, 0, 0" (Math|Vector|MakeVector 1.0 4e+01 4e+01)) "AlwaysSpawn" 0 0))
    (:then_1
      (for _index (range 0 (/ (Variables|Default|GetNumberOfTerrain) 2))
        (CallFunction|PlaceSingleTerrain)))
    (:then_2
      (CallFunction|MirrorAllTerrainOffYAxis))))

(fn DoubleMirrorTerrainPlacement
  (Utilities|FlowControl|Sequence
    (:then_0
      (Game|SpawnActorfromClass "/Game/SceneBuilder/BP_Blocker.BP_Blocker_C" (Math|Transform|MakeTransform (Variables|Default|GetBoundOrigin) "0, 0, 0" (Math|Vector|MakeVector 1.0 4e+01 4e+01)) "AlwaysSpawn" 0 0)
      (Game|SpawnActorfromClass "/Game/SceneBuilder/BP_Blocker.BP_Blocker_C" (Math|Transform|MakeTransform (Variables|Default|GetBoundOrigin) "0, 0, 0" (Math|Vector|MakeVector 4e+01 1.0 4e+01)) "AlwaysSpawn" 0 0))
    (:then_1
      (for _index (range 0 (/ (Variables|Default|GetNumberOfTerrain) 2))
        (CallFunction|PlaceSingleTerrain)))
    (:then_2
      (CallFunction|MirrorAllTerrainOffYAxis))
    (:then_3
      (CallFunction|MirrorAllTerrainOffXAxis))))

(fn MirrorAllTerrainOffXAxis
  (bind _outactors (Actor|GetAllActorsOfClass "/Game/SceneBuilder/BP_Terrain.BP_Terrain_C"))
  (for _array_element _outactors
    (Game|SpawnActorfromClass "/Game/SceneBuilder/BP_Terrain.BP_Terrain_C" (Math|Transform|MakeTransform (Math|Vector|MakeVector (.x (.location (Transformation|GetActorTransform _array_element))) (+ (.y (.location (Transformation|GetActorTransform _array_element))) (* (- (.y (Variables|Default|GetBoundOrigin)) (.y (.location (Transformation|GetActorTransform _array_element)))) 2.0)) (.z (.location (Transformation|GetActorTransform _array_element)))) (Math|Rotator|MakeRotator (.roll (.rotation (Transformation|GetActorTransform _array_element))) (.pitch (.rotation (Transformation|GetActorTransform _array_element))) (* (.yaw (.rotation (Transformation|GetActorTransform _array_element))) -1.0)) (Math|Vector|MakeVector (.x (.scale (Transformation|GetActorTransform _array_element))) (* (.y (.scale (Transformation|GetActorTransform _array_element))) -1.0) (.z (.scale (Transformation|GetActorTransform _array_element))))) "AdjustIfPossibleButDontSpawnIfColliding" 0 (Variables|/Game/SceneBuilder/BP_Terrain.BP_Terrain_C|GetTerrainName _array_element) 0)))

(fn MirrorAllTerrainOffYAxis
  (bind _outactors (Actor|GetAllActorsOfClass "/Game/SceneBuilder/BP_Terrain.BP_Terrain_C"))
  (for _array_element _outactors
    (Game|SpawnActorfromClass "/Game/SceneBuilder/BP_Terrain.BP_Terrain_C" (Math|Transform|MakeTransform (Math|Vector|MakeVector (- (.x (Variables|Default|GetBoundOrigin)) (.x (.location (Transformation|GetActorTransform _array_element)))) (.y (.location (Transformation|GetActorTransform _array_element))) (.z (.location (Transformation|GetActorTransform _array_element)))) (Math|Rotator|MakeRotator (.roll (.rotation (Transformation|GetActorTransform _array_element))) (.pitch (.rotation (Transformation|GetActorTransform _array_element))) (* (.yaw (.rotation (Transformation|GetActorTransform _array_element))) -1.0)) (Math|Vector|MakeVector (* (.x (.scale (Transformation|GetActorTransform _array_element))) -1.0) (.y (.scale (Transformation|GetActorTransform _array_element))) (.z (.scale (Transformation|GetActorTransform _array_element))))) "AdjustIfPossibleButDontSpawnIfColliding" 0 (Variables|/Game/SceneBuilder/BP_Terrain.BP_Terrain_C|GetTerrainName _array_element) 0)))

(fn CleanupTerrain
  (Utilities|FlowControl|Sequence
    (:then_0
      (bind _outactors (Actor|GetAllActorsOfClass "/Game/SceneBuilder/BP_Terrain.BP_Terrain_C"))
      (for _array_element _outactors
        (if (Utilities|IsNotWithinGameBoardBounds _array_element)
          (bind _output_get (LocalVariables|SetPiecesToDelete (Actor|GetAttachedActors _array_element true)))
          (Actor|DestroyActor _array_element)
          (for _array_element_2 _output_get
            (Actor|DestroyActor _array_element_2)))))
    (:then_1
      (bind _outactors_2 (Actor|GetAllActorsOfClass "/Game/SceneBuilder/Piece/BP_Piece.BP_Piece_C"))
      (for _array_element_3 _outactors_2
        (if (Utilities|IsNotWithinGameBoardBounds _array_element_3)
          (Actor|DestroyActor _array_element_3))))))

(fn RemoveBlockers
  (bind _outactors (Actor|GetAllActorsOfClass "/Game/SceneBuilder/BP_Blocker.BP_Blocker_C"))
  (for _array_element _outactors
    (Actor|DestroyActor _array_element)))