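; BP_Terrain is a scene-builder actor that assembles a terrain from data when play begins.
; It looks up its TerrainName row in DT_Terrain and prints an error if the row is missing.
; Each entry in the row spawns a BP_Piece with that entry's transform, tags as traits and mesh, attached to the terrain with relative rules.
; A separate function destroys its collision box component.
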(event EventBeginPlay
  (bind _returnvalue (Utilities|GetDataTableRow "/Game/SceneBuilder/DT_Terrain.DT_Terrain" (Variables|Default|GetTerrainName))
    (:then
      (for _array_element (Utilities|Struct|BreakStruct_Terrain _returnvalue)
        (CallFunction|AddPiece _array_element)))
    (:RowNotFound
      (Development|PrintString "ERROR: Terrain not found in database"))))

(event Collision|EventActorBeginOverlap
  (params (OtherActor :type Actor%20Object%20Reference)))

(event EventTick
  (params (DeltaSeconds :type Float%20%28single-precision%29)))

(fn ConstructionScript)

(fn AddPiece
  (params (TerrainPieceData :type Struct%20Piece%20Structure))
  (bind (_tags _mesh _transform) (Utilities|Struct|BreakStruct_Piece TerrainPieceData))
  (bind _returnvalue (Game|SpawnActorfromClass "/Game/SceneBuilder/Piece/BP_Piece.BP_Piece_C" _transform "Undefined" 0 _tags 0))
  (Components|StaticMesh|SetStaticMesh (Variables|/Game/SceneBuilder/Piece/BP_Piece.BP_Piece_C|GetModel _returnvalue) _mesh)
  (Transformation|AttachActorToActor _returnvalue self "None" "KeepRelative" "KeepRelative" "KeepRelative" true))

(fn DestroyCollisionBox
  (Components|DestroyComponent (Variables|Default|GetBox)))