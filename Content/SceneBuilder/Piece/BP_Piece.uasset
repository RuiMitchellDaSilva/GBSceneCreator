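; BP_Piece is a scene builder piece that shows its gameplay trait when the cursor hovers over its Model component.
; On cursor over, it prints every tag in Traits, then switches on the first tag to apply a trait-specific material to slot 0, covering types such as Structure, Low Wall and Defense.
; On cursor exit, it sets that slot to M_TraitHighlight and prints a debug message.
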(event OnBeginCursorOver(Model)
  (params (TouchedComponent :type Primitive%20Component%20Object%20Reference))
  (Utilities|FlowControl|Sequence
    (:then_0
      (for _array_element (Variables|Default|GetTraits)
        (Development|PrintString (Utilities|String|ToString(Name) (GameplayTags|GetTagName _array_element)))))
    (:then_1
      (|SwitchGameplayTag (Utilities|Array|Get(acopy) (Variables|Default|GetTraits))
        (:Structure
          (Rendering|Material|SetMaterial (Variables|Default|GetModel) 0 "/Game/SceneBuilder/Piece/MI_Structure.MI_Structure"))
        (:LowWall
          (Rendering|Material|SetMaterial (Variables|Default|GetModel) 0 "/Game/SceneBuilder/Piece/MI_LowWall.MI_LowWall"))
        (:VaultOver
          (Rendering|Material|SetMaterial (Variables|Default|GetModel) 0 "/Game/SceneBuilder/Piece/MI_VaultOver.MI_VaultOver"))
        (:NoneDetail
          (Rendering|Material|SetMaterial (Variables|Default|GetModel) 0 "/Game/SceneBuilder/Piece/MI_NoneDetail.MI_NoneDetail"))
        (:Defense
          (Rendering|Material|SetMaterial (Variables|Default|GetModel) 0 "/Game/SceneBuilder/Piece/MI_Defense.MI_Defense"))
        (:HighGround
          (Rendering|Material|SetMaterial (Variables|Default|GetModel) 0 "/Game/SceneBuilder/Piece/MI_HighGround.MI_HighGround"))
        (:Special
          (Rendering|Material|SetMaterial (Variables|Default|GetModel) 0 "/Game/SceneBuilder/Piece/MI_Special.MI_Special"))))))

(event OnEndCursorOver(Model)
  (params (TouchedComponent :type Primitive%20Component%20Object%20Reference))
  (Rendering|Material|SetMaterial (Variables|Default|GetModel) 0 "/Game/SceneBuilder/Piece/M_TraitHighlight.M_TraitHighlight")
  (Development|PrintString "Turn off highlight"))

(event EventBeginPlay)

(event Collision|EventActorBeginOverlap
  (params (OtherActor :type Actor%20Object%20Reference)))

(event EventTick
  (params (DeltaSeconds :type Float%20%28single-precision%29)))

(fn ConstructionScript)