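; GM_BoardViewer is the scene builder game mode that persists placed BP_Terrain actors in a single save slot, "Save1".
; On BeginPlay it respawns terrain from the saved name and transform entries, or creates an empty save if none exists.
; SaveGame overwrites those entries with every BP_Terrain currently in the level.
; LoadGame simply restarts the level, so BeginPlay rebuilds the saved scene.
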(event Custom|SaveGame
  (Utilities|Array|Clear (Variables|Default|GetTerrainToSave))
  (bind _returnvalue (SaveGame|LoadGamefromSlot "Save1"))
  (bind _asbp_save_object (Utilities|Casting|CastToBP_SaveObject _returnvalue))
  (bind _outactors (Actor|GetAllActorsOfClass "/Game/SceneBuilder/BP_Terrain.BP_Terrain_C"))
  (for _array_element _outactors
    (Utilities|Array|Add (Variables|Default|GetTerrainToSave) (Utilities|Struct|MakeStruct_TerrainSave (Variables|/Game/SceneBuilder/BP_Terrain.BP_Terrain_C|GetTerrainName _array_element) (Transformation|GetActorTransform _array_element))))
  (Variables|/Game/SceneBuilder/BP_SaveObject.BP_SaveObject_C|SetSceneTerrain _asbp_save_object (Variables|Default|GetTerrainToSave))
  (SaveGame|SaveGametoSlot _asbp_save_object "Save1"))

(event Custom|LoadGame
  (Development|ExecuteConsoleCommand "RestartLevel" 0))

(event EventBeginPlay
  (bind _returnvalue (SaveGame|DoesSaveGameExist "Save1"))
  (if _returnvalue
    (bind _returnvalue_2 (SaveGame|LoadGamefromSlot "Save1"))
    (bind _asbp_save_object (Utilities|Casting|CastToBP_SaveObject _returnvalue_2))
    (for _array_element (Variables|/Game/SceneBuilder/BP_SaveObject.BP_SaveObject_C|GetSceneTerrain _asbp_save_object)
      (Game|SpawnActorfromClass "/Game/SceneBuilder/BP_Terrain.BP_Terrain_C" (.Transform (Utilities|Struct|BreakStruct_TerrainSave _array_element)) "Undefined" 0 (.TerrainName (Utilities|Struct|BreakStruct_TerrainSave _array_element)) 0))
    (else
      (bind _returnvalue_3 (SaveGame|CreateSaveGameObject "/Game/SceneBuilder/BP_SaveObject.BP_SaveObject_C"))
      (SaveGame|SaveGametoSlot _returnvalue_3 "Save1")
      (Development|PrintString "NewSameSlotCreated"))))

(fn ConstructionScript)