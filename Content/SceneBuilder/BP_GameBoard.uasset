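; BP_GameBoard is the game board actor, which creates two player zones when play begins.
; SetupPlayerZones spawns two BP_Zone actors on either side of the Board along X, offset by ZoneXDelta and scaled from the board size constants.
; The zone on the negative X side gets an explicit ZoneOwnership, while the other keeps the default.
; BeginPlay also prints TerranBuilder's display name for debugging.
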(event Custom|DEBUG_PrintChildName
  (Development|PrintString (Utilities|GetDisplayName (Variables|Default|GetTerranBuilder))))

(event EventBeginPlay
  (CallFunction|DEBUGPrintChildName)
  (CallFunction|SetupPlayerZones))

(event Collision|EventActorBeginOverlap
  (params (OtherActor :type Actor%20Object%20Reference)))

(event EventTick
  (params (DeltaSeconds :type Float%20%28single-precision%29)))

(fn ConstructionScript)

(fn SetupPlayerZones
  (bind _board (Variables|Default|GetBoard))
  (bind _board_size_x (Variables|Default|GetBOARD_SIZE_X))
  (bind _board_size_y (Variables|Default|GetBOARD_SIZE_Y))
  (bind _returnvalue (Transformation|GetWorldLocation _board))
  (bind _returnvalue_2 (/ _board_size_x 4.0))
  (bind _returnvalue_3 (/ _board_size_y 2.0))
  (Game|SpawnActorfromClass "/Game/SceneBuilder/BP_Zone.BP_Zone_C" (Math|Transform|MakeTransform (Math|Vector|MakeVector (+ (.x _returnvalue) (Variables|Default|GetZoneXDelta)) (.y _returnvalue) (.z _returnvalue)) "0, 0, 0" (Math|Vector|MakeVector _returnvalue_2 _returnvalue_3 1.0)) "Undefined" 0 "NewEnumerator0" 0)
  (Game|SpawnActorfromClass "/Game/SceneBuilder/BP_Zone.BP_Zone_C" (Math|Transform|MakeTransform (Math|Vector|MakeVector (- (.x _returnvalue) (Variables|Default|GetZoneXDelta)) (.y _returnvalue) (.z _returnvalue)) "0, 0, 0" (Math|Vector|MakeVector _returnvalue_2 _returnvalue_3 1.0)) "Undefined" 0 "NewEnumerator1" 0))